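; BP_Enemy is a sprite-based melee enemy that chases the first-person player and hurts them on contact.
; PawnSensing spots the player and triggers AI MoveTo, after which Tick keeps the actor's yaw turned toward the player, billboard-style.
; A box overlap applies damage to the player.
; Incoming damage drains Health; at zero, movement deactivates and death and corpse flipbooks play before the actor is destroyed.
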(event `self.PawnSensing.OnSeePawn`
  (params (Pawn :type "Pawn Object Reference"))
  ;[0 0.9272 1 0.5] IA
  (bind _asbp_first_person_character (cast `/Game/FirstPerson/Blueprints/BP_FirstPersonCharacter` Pawn))
  (set `self.CanSeePlayer` true)
  (`|AIMoveTo` self (0.0 0.0 0.0) _asbp_first_person_character))

(event `self.ReceiveTick`
  (params (DeltaSeconds :type "Float (single-precision)"))
  (bind (_returnvalue_roll _returnvalue_pitch _returnvalue_yaw) (`KismetMathLibrary.BreakRotator` (`KismetMathLibrary.FindLookAtRotation` (`self.K2_GetActorLocation`) (`self.K2_GetActorLocation` (`GameplayStatics.GetPlayerCharacter` 0)))))
  ;[0.4167 0.3583 0 0.5] Sprite Rotation
  (if (`self.CanSeePlayer`)
    (`self.K2_SetActorRotation` (`KismetMathLibrary.MakeRotator` 0.0 0.0 _returnvalue_yaw))))

(event `self.ReceiveAnyDamage`
  (params (Damage :type "Float (single-precision)") (DamageType :type "DamageType Object Reference") (InstigatedBy :type "Controller Object Reference") (DamageCauser :type "Actor Object Reference"))
  (bind _paperflipbook (`self.PaperFlipbook`))
  ;[0.000231 0.1042 0 0.5] Health Enemy
  (bind _output_get (set `self.Health` (- (`self.Health`) Damage)))
  (if (<= _output_get 0.0)
    (`ActorComponent.Deactivate` (`self.CharacterMovement`))
    (`PaperFlipbookComponent.SetFlipbook` _paperflipbook "/Game/Blueprints/Enemy/Melee_Enemy/meleedeath1.meleedeath1")
    (`KismetSystemLibrary.Delay` (`PaperFlipbookComponent.GetFlipbookLength` _paperflipbook))
    (`PaperFlipbookComponent.SetFlipbook` (`self.PaperFlipbook`) "/Game/Blueprints/Enemy/Melee_Enemy/Dead01.Dead01")
    (`KismetSystemLibrary.Delay` 4.0)
    (`self.K2_DestroyActor`)))

(event `self.Box.OnComponentBeginOverlap`
  (params (OverlappedComponent :type "PrimitiveComponent Object Reference") (OtherActor :type "Actor Object Reference") (OtherComp :type "PrimitiveComponent Object Reference") (OtherBodyIndex :type Integer) (bFromSweep :type Boolean) (SweepResult :type "HitResult Structure (by ref)"))
  (bind _asbp_first_person_character (cast `/Game/FirstPerson/Blueprints/BP_FirstPersonCharacter` OtherActor))
  (`GameplayStatics.ApplyDamage` _asbp_first_person_character 10.0 null self "/Script/Engine.DamageType"))

(fn `UserConstructionScript`)