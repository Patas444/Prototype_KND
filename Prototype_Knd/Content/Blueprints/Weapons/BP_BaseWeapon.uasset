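; BP_BaseWeapon is a base hitscan weapon with empty ShootWeapon and StopShooting events.
; Fireweapon spends one Ammo, then line traces forward from the Linetrace component against world and pawn objects, ignoring itself and the player, with debug drawing.
; A hit applies WeaponDamage and refreshes the owning BP_FirstPersonCharacter's HUD ammo text, so misses leave the display unchanged.
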(event `ShootWeapon`)

(event `StopShooting`)

(fn `Fireweapon`
  (bind _returnvalue (`SceneComponent.K2_GetComponentLocation` (`self.Linetrace`)))
  (bind _output_get (set `self.Ammo` (`self.Ammo`)))
  (if (> _output_get 0)
    (set `self.Ammo` (- (`self.Ammo`) 1))
    (bind (_outhit _returnvalue_2) (`KismetSystemLibrary.LineTraceSingleForObjects` _returnvalue (+ _returnvalue (* (`KismetMathLibrary.GetForwardVector` (`SceneComponent.K2_GetComponentRotation` (`self.Linetrace`))) (`self.Linetracedistance`))) (`|MakeArray` "ObjectTypeQuery1" "ObjectTypeQuery2" "ObjectTypeQuery3" :!type "EObjectTypeQuery Enum") false (`|MakeArray` self (`GameplayStatics.GetPlayerCharacter` 0) :!type "Actor Object Reference") "ForDuration"))
    (if _returnvalue_2
      (`GameplayStatics.ApplyDamage` (`.HitActor` (`GameplayStatics.BreakHitResult` _outhit)) (`self.WeaponDamage`))
      (bind _asbp_first_person_character (cast `/Game/FirstPerson/Blueprints/BP_FirstPersonCharacter` (`self.GetOwner`)))
      (`/Game/Blueprints/UI/WBP_HUD.UpdateAmmoText` (`/Game/FirstPerson/Blueprints/BP_FirstPersonCharacter.HUDWidget` _asbp_first_person_character)))))

(fn `UserConstructionScript`)