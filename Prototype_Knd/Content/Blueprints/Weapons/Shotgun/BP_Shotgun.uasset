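; BP_Shotgun is a shotgun weapon Blueprint that fires and animates its sprite through a Paper2D flipbook component.
; ShootWeapon passes a DoOnce gate, calls Fireweapon, plays the fire flipbook for its length, then switches back to idle.
; The gate blocks further shots until ResetWeapon reopens it, as the delay does not reset it.
; The construction script only runs the parent's.
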(event `self.ShootWeapon`
  (bind _weaponflipbook (`self.WeaponFlipbook`))
  (`/Engine/EditorBlueprintResources/StandardMacros.DoOnce` false :!label _label
    (:`Completed`
      (`self.Fireweapon`)
      (`PaperFlipbookComponent.SetFlipbook` _weaponflipbook "/Game/Blueprints/Weapons/Shotgun/shotgunFire.shotgunFire")
      (`KismetSystemLibrary.Delay` (`PaperFlipbookComponent.GetFlipbookLength` _weaponflipbook))
      (`PaperFlipbookComponent.SetFlipbook` (`self.WeaponFlipbook`) "/Game/Blueprints/Weapons/Shotgun/shotgunIdle.shotgunIdle"))))

(event `ResetWeapon`
  (goto _label :!via `Reset`))

(fn `UserConstructionScript`
  (`parent.UserConstructionScript`))