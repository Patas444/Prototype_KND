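; BP_AmmoItem is an ammo pickup that adds to the player's main weapon ammo.
; Each tick it yaws toward the player character so its sprite faces them, billboard style.
; When BP_FirstPersonCharacter overlaps its sphere, it adds AmmoAmount to MainWeapon's Ammo, plays a 2D heal sound and destroys itself.
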(event `self.ReceiveTick`
  (params (DeltaSeconds :type "Float (single-precision)"))
  (bind (_returnvalue_roll _returnvalue_pitch _returnvalue_yaw) (`KismetMathLibrary.BreakRotator` (`KismetMathLibrary.FindLookAtRotation` (`self.K2_GetActorLocation`) (`self.K2_GetActorLocation` (`GameplayStatics.GetPlayerCharacter` 0)))))
  ;[0.4167 0.3583 0 0.5] Sprite Rotation
  (`self.K2_SetActorRotation` (`KismetMathLibrary.MakeRotator` 0.0 0.0 _returnvalue_yaw)))

(event `self.ReceiveBeginPlay`
  (`self.SetActorHiddenInGame` false))

(event `self.Sphere1.OnComponentBeginOverlap`
  (params (OverlappedComponent :type "PrimitiveComponent Object Reference") (OtherActor :type "Actor Object Reference") (OtherComp :type "PrimitiveComponent Object Reference") (OtherBodyIndex :type Integer) (bFromSweep :type Boolean) (SweepResult :type "HitResult Structure (by ref)"))
  (bind _asbp_first_person_character (cast `/Game/FirstPerson/Blueprints/BP_FirstPersonCharacter` OtherActor))
  (bind _mainweapon (`/Game/FirstPerson/Blueprints/BP_FirstPersonCharacter.MainWeapon` _asbp_first_person_character))
  (set `/Game/Blueprints/Weapons/BP_BaseWeapon.Ammo` (+ (`/Game/Blueprints/Weapons/BP_BaseWeapon.Ammo` _mainweapon) (`self.AmmoAmount`)) _mainweapon)
  (`GameplayStatics.PlaySound2D` "/Game/Blueprints/Items/Undertale_Sound_Effect_-_Heal.Undertale_Sound_Effect_-_Heal" 1.0 1.0 0.0 null null)
  (`self.K2_DestroyActor`))

(fn `UserConstructionScript`)